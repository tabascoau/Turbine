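; Turbine actor that spins its fan blade and pushes physics objects in a box range, which the construction script sizes and offsets from its range variables.
; While anything overlaps the box, Tick casts a grid of debug-drawn Visibility traces from the actor's plane along world Z.
; Simulating hits receive force at the impact point, aimed between actor up and the inverted surface normal, scaled by their alignment.
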(event EventTick
  (params (DeltaSeconds :type Float%20%28single-precision%29))
  (bind _returnvalue (Transformation|GetActorTransform))
  (bind _returnvalue_2 (Transformation|GetActorUpVector))
  (bind _distbetweenforcelines (Variables|Default|GetDistBetweenForceLines))
  (Transformation|AddWorldRotation (Variables|Default|GetSM_FanBlade) "0.000000,20.000000, 0" false false)
  (if (> (Utilities|Array|Length (Class|PrimitiveComponent|GetOverlappingComponents (Variables|Default|GetRange))) 0)
    (for _index (range 0 (Math|Float|Truncate (/ (Variables|Default|GetRangeX) (Variables|Default|GetDistBetweenForceLines))))
      (for _index_2 (range 0 (Math|Float|Truncate (/ (Variables|Default|GetRangeY) (Variables|Default|GetDistBetweenForceLines))))
        (bind (_outhit _returnvalue_3) (Collision|LineTraceByChannel (Math|Transform|TransformLocation _returnvalue (Math|Vector|MakeVector (- (* _index_2 _distbetweenforcelines) (/ (Variables|Default|GetRangeX) 2.0)) (- (* _index _distbetweenforcelines) (/ (Variables|Default|GetRangeY) 2.0)) 0.0)) (Math|Transform|TransformLocation _returnvalue (+ (Math|Vector|MakeVector (- (* _index_2 _distbetweenforcelines) (/ (Variables|Default|GetRangeX) 2.0)) (- (* _index _distbetweenforcelines) (/ (Variables|Default|GetRangeY) 2.0)) 0.0) (Math|Vector|MakeVector 0.0 0.0 (Variables|Default|GetRangeZ)))) "TraceTypeQuery1" false 0 "ForOneFrame"))
        (if _returnvalue_3
          (if (Physics|IsSimulatingPhysics (.HitComponent (Collision|BreakHitResult _outhit)) "None")
            (Class|PrimitiveComponent|AddForceatLocation (.HitComponent (Collision|BreakHitResult _outhit)) (* (Math|Vector|Normalize (+ _returnvalue_2 (Math|Vector|NegateVector (.ImpactNormal (Collision|BreakHitResult _outhit))))) (* (Math|Float|Absolute(Float) (Math|Vector|DotProduct _returnvalue_2 (Math|Vector|NegateVector (.ImpactNormal (Collision|BreakHitResult _outhit))))) (Variables|Default|GetMaxForce))) (.ImpactPoint (Collision|BreakHitResult _outhit)) "None")))))))

(fn ConstructionScript
  (bind _range (Variables|Default|GetRange))
  (Components|Box|SetBoxExtent _range (Math|Vector|MakeVector (/ (Variables|Default|GetRangeX) 2.0) (/ (Variables|Default|GetRangeY) 2.0) (/ (Variables|Default|GetRangeZ) 2.0)) true)
  (Transformation|SetRelativeLocation (Variables|Default|GetRange) (Math|Vector|MakeVector 0.0 0.0 (.z (Variables|/Script/Engine.BoxComponent|GetBoxExtent _range))) false false))